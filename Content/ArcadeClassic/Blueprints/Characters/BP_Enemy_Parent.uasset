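; Parent Blueprint for arcade enemies that kill the player on contact, or get eaten while vulnerable after a power pellet.
; A timeline drives two vulnerable phases by toggling visual component visibility, then restores the regular state.
; Overlap with the player either plays death effects, hides the enemy and ignores Pawn collision, or signals a kill.
; Dispatchers announce player kills and vulnerability changes, the latter letting the GameMode switch music.
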(event OnComponentBeginOverlap(Player_Collision)
  (params (OverlappedComponent :type Primitive%20Component%20Object%20Reference) (OtherActor :type Actor%20Object%20Reference) (OtherComp :type Primitive%20Component%20Object%20Reference) (OtherBodyIndex :type Integer) (bFromSweep :type Boolean) (SweepResult :type Hit%20Result%20Structure%20%28by%20ref%29))
  ;[0 1 0.08243] Enemy collides with player
  (bind _asbp_player (Utilities|Casting|CastToBP_Player OtherActor)) ; Did collision with player occur?
  (Utilities|IsValid _asbp_player
    (:Is%20Valid
      (if (Variables|EnemyVulnerable|GetbIsVulnerable) ; Am I vulnerable?
        (CallFunction|EnemyEatenFX)
        (Collision|SetCollisionResponsetoChannel (Variables|Default|GetPlayer_Collision) "ECC_Pawn" "ECR_Ignore")
        (else
          (Default|CallKilledPlayer))))))

(event Custom|POWER%20PELLET%20EATEN
  ;[0 1 0.08243] Vulnerability Sequence
  (Variables|EnemyVulnerable|SetbIsVulnerable true)
  (Default|CallVulnerable) ; Calls Event in GameMode BP to alter game's music
  (Timeline|VulnerabilitySequence PlayFromStart
    (:Finished
      (CallFunction|EnemyStateRegular)
      (Variables|EnemyVulnerable|SetbIsVulnerable false)
      (Default|CallNotVulnerable) ; Messages GameMode BP to alter music
    )
    (:StartPhaseOne
      (CallFunction|EnemyStateVulnerable01))
    (:StartPhaseTwo
      (if (Variables|EnemyVulnerable|GetbIsVulnerable) ; Is enemy still vulnerable or was it eaten?
        (CallFunction|EnemyStateVulnerable02)))))

(fn ConstructionScript)

(fn EnemyStateRegular
  (Rendering|SetVisibility (Variables|Default|GetEnemy_Vulnerable_01) false false)
  (Rendering|SetVisibility (Variables|Default|GetEnemy_Down) true false))

(fn EnemyStateVulnerable01
  (Rendering|SetVisibility (Variables|Default|GetEnemy_Vulnerable_02) false false)
  (Rendering|SetVisibility (Variables|Default|GetEnemy_Vulnerable_01) true false))

(fn EnemyStateVulnerable02
  (Rendering|SetVisibility (Variables|Default|GetEnemy_Down) false false)
  (Rendering|SetVisibility (Variables|Default|GetEnemy_Vulnerable_02) true false))

(fn EnemyEatenFX
  (Effects|SpawnEmitteratLocation "/Game/ArcadeClassic/Particles/P_Death.P_Death" (Transformation|GetWorldLocation (Variables|Collision|GetCapsuleComponent)))
  (Audio|PlaySound2D "/Game/ArcadeClassic/Audio/SFX_EatEnemy_Cue.SFX_EatEnemy_Cue" 1.0 1.0 0.0 0 0)
  (Rendering|SetActorHiddenInGame true))