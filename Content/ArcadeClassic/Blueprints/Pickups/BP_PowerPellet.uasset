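; BP_PowerPellet is the power pellet pickup, consumed when BP_Player overlaps its mesh.
; On pickup it plays a 2D sound, activates the eaten VFX, removes the mesh and glow, then destroys the actor after a short delay.
; A second sequence branch immediately calls ATEPELLET on BP_GameMode_GamePlay to decrement the level's pellet count, without waiting for that delay.
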(event OnComponentBeginOverlap(SM_PowerPellet)
  (params (OverlappedComponent :type Primitive%20Component%20Object%20Reference) (OtherActor :type Actor%20Object%20Reference) (OtherComp :type Primitive%20Component%20Object%20Reference) (OtherBodyIndex :type Integer) (bFromSweep :type Boolean) (SweepResult :type Hit%20Result%20Structure%20%28by%20ref%29))
  (Utilities|Casting|CastToBP_Player OtherActor)
  (Utilities|FlowControl|Sequence
    (:then_0
      ;[0 1 0.05132] Power Pellet Eaten Handling
      (Audio|PlaySound2D "/Game/ArcadeClassic/Audio/SFX_EatSpecial_Cue.SFX_EatSpecial_Cue" 1.0 1.0 0.0 0 0)
      (Components|Activation|Activate (Variables|Default|GetVFX_PowerPellet_Eaten) false)
      (Components|DestroyComponent (Variables|Default|GetSM_PowerPellet))
      (Utilities|FlowControl|Delay 5.0)
      (Actor|DestroyActor))
    (:then_1
      ;[0 1 0.1175] GameMode BP - Decrement Level's Pellet Count
      (bind _asbp_game_mode_game_play (Utilities|Casting|CastToBP_GameMode_GamePlay (Game|GetGameMode)))
      (Default|ATEPELLET _asbp_game_mode_game_play))))

(fn ConstructionScript)