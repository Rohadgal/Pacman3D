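; Gameplay game mode for an arcade game, handling the intro camera move and a bonus item spawn.
; On BeginPlay it disables player input, blends the view to a newly spawned gameplay camera, then after a delay restores input and allows BP_Player to move.
; In parallel, after a random delay, it spawns one cherry, orange or speed power-up at one of two locations, without repeating.
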(event EventBeginPlay
  (bind _returnvalue (Game|GetPlayerCharacter 0))
  (bind _goodiespawn_01 (Variables|Goodies|GetGoodieSpawn_01))
  (bind _goodiespawn_02 (Variables|Goodies|GetGoodieSpawn_02))
  (bind _array (Utilities|Array|MakeArray _goodiespawn_01 _goodiespawn_02))
  (Utilities|FlowControl|Sequence
    (:then_3
      ;[1 0.8425 0] GamePlay Camera
      (Input|DisableInput (Game|GetPlayerCharacter 0) (Game|GetPlayerController 0))
      (bind _returnvalue_2 (Game|SpawnActorfromClass "/Script/Engine.CameraActor" (Math|Transform|MakeTransform (Variables|Camera|GetCamGamePlay_LOC) (Variables|Camera|GetCamGamePlay_ROT) "1,1,1") "Undefined" 0 0))
      (Game|Player|SetViewTargetwithBlend (Game|GetPlayerController 0) _returnvalue_2 6.8 "VTBlend_Linear" 0.0 false)
      (Utilities|FlowControl|Delay 7.0)
      (Input|EnableInput _returnvalue (Game|GetPlayerController 0))
      (bind _asbp_player (Utilities|Casting|CastToBP_Player _returnvalue))
      (Variables|/Game/ArcadeClassic/Blueprints/Characters/BP_Player.BP_Player_C|SetbAllowedToMove _asbp_player true))
    (:then_5
      ;[0 1 0.1024] Fruit / Power-Up Spawn
      (Utilities|FlowControl|Delay (Math|Random|RandomFloatinRange 25.0 5e+01))
      (bind _output_get (Variables|Goodies|SetGoodieSpawnLocales _array))
      (switch int (Math|Random|RandomIntegerinRange 0 2)
        (:0
          (Game|SpawnActorfromClass "/Game/ArcadeClassic/Blueprints/Pickups/BP_Food_Cherry.BP_Food_Cherry_C" (Math|Conversions|ToTransform(Vector) (Utilities|Array|Get(acopy) _output_get (Math|Random|RandomIntegerinRange 0 (- (Utilities|Array|Length _array) 1)))) "Undefined" 0 0))
        (:1
          (Game|SpawnActorfromClass "/Game/ArcadeClassic/Blueprints/Pickups/BP_Food_Orange.BP_Food_Orange_C" (Math|Conversions|ToTransform(Vector) (Utilities|Array|Get(acopy) _output_get (Math|Random|RandomIntegerinRange 0 (- (Utilities|Array|Length _array) 1)))) "Undefined" 0 0))
        (:2
          (Game|SpawnActorfromClass "/Game/ArcadeClassic/Blueprints/Pickups/BP_PowerUp_Speed.BP_PowerUp_Speed_C" (Math|Conversions|ToTransform(Vector) (Utilities|Array|Get(acopy) _output_get (Math|Random|RandomIntegerinRange 0 (- (Utilities|Array|Length _array) 1)))) "Undefined" 0 0))))))

(fn ConstructionScript)